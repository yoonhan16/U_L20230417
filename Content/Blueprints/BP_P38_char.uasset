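; Player-controlled P-38 aircraft Blueprint that constantly flies forward while the player steers its pitch and roll.
; Tick feeds the actor's forward vector into movement input and spins the left and right propellers through a shared RotatePropeller function.
; Pitch and Roll axis events apply clamped, delta-time-scaled local rotations at the player rotate speed.
; An unconnected local-offset movement and delay remain unused in the graph.
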(event `self.ReceiveTick`
  (params (DeltaSeconds :type "Float (single-precision)"))
  (`|ExecutionSequence`
    (:`then_0`
      (`self.AddMovementInput` (`self.GetActorForwardVector`)))
    (:`then_1`
      ;[1 1 1] 좌측 프로펠러 회전
      (`self.Rotate Propeller` (`self.P-38_Left_Propeller`)))
    (:`then_2`
      ;[1 1 1] 우측 프로펠러 회전
      (`self.Rotate Propeller` (`self.P-38_Right_Propeller`)))))

(event `InputAxis|Pitch`
  (params (AxisValue :type "Float (single-precision)"))
  ;[1 1 1] Pitch Rotate
  (`self.K2_AddActorLocalRotation` (`KismetMathLibrary.MakeRotator` 0.0 (* (`KismetMathLibrary.FClamp` AxisValue -1.0) (`GameplayStatics.GetWorldDeltaSeconds`) (`self.Player Rotate Speed`)))))

(event `InputAxis|Roll`
  (params (AxisValue :type "Float (single-precision)"))
  ;[1 1 1] Roll Rotate
  (`self.K2_AddActorLocalRotation` (`KismetMathLibrary.MakeRotator` (* (`KismetMathLibrary.FClamp` AxisValue -1.0) (`GameplayStatics.GetWorldDeltaSeconds`) (`self.Player Rotate Speed`)))))

(fn `Rotate Propeller`
  (params (Where :type "StaticMeshComponent Object Reference"))
  (`SceneComponent.K2_AddRelativeRotation` Where (`KismetMathLibrary.MakeRotator` (* (`GameplayStatics.GetWorldDeltaSeconds`) (`self.Propeller Rotation Speed`))) false false))

(fn `UserConstructionScript`)